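; Game instance Blueprint that handles PlayFab login for the game.
; CustomLogin sets the PlayFab title ID, then logs in with a hardcoded custom ID, creating the account if needed.
; PlayfabLogin signs in with a supplied username and password without setting the title ID itself.
; LoginSuccess and LoginFailure handlers only print the outcome, and Init is empty.
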(event `CustomLogin`
  (`PlayFabUtilities.setPlayFabSettings` "562CF")
  (`PlayFabClientAPI.LoginWithCustomID` (make `ClientLoginWithCustomIDRequest` true "PlayfabSetup") (`|CreateDelegate` :!event `LoginSuccess`) (`|CreateDelegate` :!event `LoginFailure`)))

(event `self.ReceiveInit`)

(event `/Game/Blueprints/Interfaces/BPI_GameInstance.PlayfabLogin`
  (params (Username :type String) (Password :type String))
  (`PlayFabClientAPI.LoginWithPlayFab` (make `ClientLoginWithPlayFabRequest` null null Password Username) (`|CreateDelegate` :!event `LoginSuccess`) (`|CreateDelegate` :!event `LoginFailure`)))

(event `LoginSuccess`
  (params (result :type "ClientLoginResult Structure") (customData :type "Object Object Reference"))
  (`KismetSystemLibrary.PrintString` "Login Succeeded" true true (struct :`G` 0.66 :`B` 1.0 :`A` 1.0) 5.0))

(event `LoginFailure`
  (params (error :type "PlayFabError Structure") (customData :type "Object Object Reference"))
  (`KismetSystemLibrary.PrintString` "Login Failed" true true (struct :`R` 1.0 :`A` 1.0) 5.0))